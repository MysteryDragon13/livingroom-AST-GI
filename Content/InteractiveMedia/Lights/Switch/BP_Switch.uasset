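; BP_Switch is a light switch that controls an array of linked lamps.
; TurnLightsOn and TurnLightsOff set every lamp on or off, while Interact toggles each lamp individually through its own ToggleLight.
; The construction script also calls ToggleLight on every linked lamp, so their state flips whenever the switch is constructed.
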(event Custom|TurnLightsOn
  (for _array_element (Variables|Default|GetLamp)
    (Default|TurnLighton _array_element)))

(event Custom|TurnLightsOff
  (for _array_element (Variables|Default|GetLamp)
    (Default|TurnLightOff _array_element)))

(event EventInteract
  (for _array_element (Variables|Default|GetLamp)
    (Default|ToggleLight _array_element)))

(fn ConstructionScript
  (for _array_element (Variables|Default|GetLamp)
    (Default|ToggleLight _array_element)))