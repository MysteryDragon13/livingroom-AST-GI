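; BP_InteractiveLamp is an interactive lamp whose spotlight can be switched on, off or temporarily toggled.
; The construction script sets the spotlight's initial visibility from IsOn, and separate events force it on or off.
; Interact flips the visibility through ToggleLight, then flips it again after a short fixed delay.
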(event Custom|TurnLightOn
  (Rendering|SetVisibility (Variables|Default|GetSpotLight) true false))

(event Custom|TurnLightOff
  (Rendering|SetVisibility (Variables|Default|GetSpotLight) false false))

(event EventInteract
  (CallFunction|ToggleLight)
  (Utilities|FlowControl|Delay 5.0)
  (CallFunction|ToggleLight))

(fn ConstructionScript
  (Rendering|SetVisibility (Variables|Default|GetSpotLight) (Variables|Default|GetbIsOn?) false))

(fn ToggleLight
  (Rendering|ToggleVisibility (Variables|Default|GetSpotLight) false))