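; Pawn piece for a self-playing chess display, extending the shared attack and move flow with en passant and promotion.
; Special-move events store the capture square or promotion type, then attack; the attack-finished event picks the matching board update.
; En passant removes the bypassed piece, while promotion activates a despawn effect and delegates replacement to an event.
; Moves are built as "moves" strings that drive the next move.
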(event Custom|PawnPromotion
  (params (Destination :type Vector) (StartSquare :type String) (TargetSquare :type String) (Promotion :type String))
  (Variables|Default|SetPromotion Promotion)
  (CallFunction|Attack Destination StartSquare TargetSquare))

(event Custom|EnPassant
  (params (Destination :type Vector) (StartSquare :type String) (TargetSquare :type String) (EnPassantSquare :type String))
  (Variables|Default|SetEnPassantSquare EnPassantSquare)
  (CallFunction|Attack Destination StartSquare TargetSquare))

(event EventBeginPlay
  (|CallParentFunction) ; This node is disabled and will not be called.\nDrag off pins to build functionality.
)

(event Collision|EventActorBeginOverlap
  (params (OtherActor :type Actor%20Object%20Reference))
  (|CallParentFunction OtherActor) ; This node is disabled and will not be called.\nDrag off pins to build functionality.
)

(event EventTick
  (params (DeltaSeconds :type Float%20%28single-precision%29))
  (|CallParentFunction DeltaSeconds) ; This node is disabled and will not be called.\nDrag off pins to build functionality.
)

(event EventOnAttackFinished
  (params (StartField :type String) (TargetField :type String))
  (if (Utilities|Enum|NotEqual(Enum) (Variables|Default|GetEnPassantSquare) "-")
    (bind _move (CallFunction|UpdateBoardonEnPassant StartField TargetField))
    (Variables|Default|SetEnPassantSquare "-")
    (CallFunction|InitiateNextMove _move)
    (elif (Utilities|Enum|NotEqual(Enum) (Variables|Default|GetPromotion) "-")
      (CallFunction|UpdateBoardonPawnPromotion StartField TargetField)
      (else
        (bind _move_2 (CallFunction|UpdateBoardandGetMove StartField TargetField))
        (CallFunction|InitiateNextMove _move_2)))))

(fn ConstructionScript
  (|CallParentFunction))

(fn UpdateBoardonEnPassant
  (params (StartField :type String) (TargetField :type String))
  (Utilities|FlowControl|Sequence
    (:then_0
      ;[1 1 1] First we need to save the ChessPiece Reference of the starting position and then set the field to empty
      (bind _field (Utilities|GetSquarebyName StartField)
        (:Is%20Valid
          (LocalVariables|SetChessPieceToMove (Variables|/Game/InteractiveMedia/SelfPlayingChess/Board/BP_SelfPlayingChessTile.BP_SelfPlayingChessTile_C|GetPresentChesspiece _field))
          (Variables|/Game/InteractiveMedia/SelfPlayingChess/Board/BP_SelfPlayingChessTile.BP_SelfPlayingChessTile_C|SetPresentChesspiece _field 0))))
    (:then_1
      ;[1 1 1] Then we need to set the ChessPiece at the target field to the one from the starting position
      (bind _field_2 (Utilities|GetSquarebyName TargetField)
        (:Is%20Valid
          (Variables|/Game/InteractiveMedia/SelfPlayingChess/Board/BP_SelfPlayingChessTile.BP_SelfPlayingChessTile_C|SetPresentChesspiece _field_2 (LocalVariables|GetChessPieceToMove)))))
    (:then_2
      ;[1 1 1] Together with the move we need to trigger the captured event for the EnPassant field
      (bind _field_3 (Utilities|GetSquarebyName (Variables|Default|GetEnPassantSquare))
        (:Is%20Valid
          (Default|Captured (Variables|/Game/InteractiveMedia/SelfPlayingChess/Board/BP_SelfPlayingChessTile.BP_SelfPlayingChessTile_C|GetPresentChesspiece _field_3))
          (Variables|/Game/InteractiveMedia/SelfPlayingChess/Board/BP_SelfPlayingChessTile.BP_SelfPlayingChessTile_C|SetPresentChesspiece _field_3 0))))
    (:then_3
      (return (Utilities|String|Append " moves " StartField TargetField)))))

(fn UpdateBoardonPawnPromotion
  (params (StartField :type String) (TargetField :type String%20%28by%20ref%29))
  ;[1 1 1] We just need to set the ChessPiece on the starting field to empty, the rest will be handled by the event
  (bind _field (Utilities|GetSquarebyName StartField)
    (:Is%20Valid
      (Variables|/Game/InteractiveMedia/SelfPlayingChess/Board/BP_SelfPlayingChessTile.BP_SelfPlayingChessTile_C|SetPresentChesspiece _field 0)
      (Components|Activation|SetActive (Variables|Default|GetDespawn) true false)
      (bind _field_2 (Utilities|GetSquarebyName TargetField)
        (:Is%20Valid
          (CallFunction|OnPawnPromotionInitiated self _field_2 (Variables|Default|GetPromotion) (Utilities|String|Append " moves " StartField TargetField (Variables|Default|GetPromotion))))))))