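; Chess piece actor for a self-playing chessboard that animates its moves, keeps the board's fields current and passes the move string to the board to start the next turn.
; Timelines slide the piece toward its target or lift, move and land it for jumps.
; An attacking piece captures opposite-colored pieces on overlap, triggering particles and delayed destruction.
; En passant, castling and promotion entry events are empty stubs, with helpers for promotion spawning and castling updates.
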(event Custom|Castle
  (params (TargetLocationKing :type Vector) (StartSquareKing :type String) (TargetSquareKing :type String) (Rook :type BP%20Self%20Playing%20Chess%20Piece%20Object%20Reference) (TargetLocationRook :type Vector) (StartSquareRook :type String) (TargetSquareRook :type String) (Move :type String))
  ;[1 1 1] Events for Special Cases
)

(event Custom|EnPassant
  (params (Destination :type Vector) (StartSquare :type String) (TargetSquare :type String) (EnPassantSquare :type String))
  ;[1 1 1] Events for Special Cases
)

(event Custom|PawnPromotion
  (params (Destination :type Vector) (StartSquare :type String) (TargetSquare :type String) (Promotion :type String))
  ;[1 1 1] Events for Special Cases
)

(event Custom|Attack
  (params (Target :type Vector) (StartField :type String) (TargetField :type String))
  ;[1 1 1] Attack the given field (Has to be an event, because timed functions are not allowed in functions - only in  Macros)
  (Variables|Default|SetAttacking true)
  (CallFunction|PrepareMove Target)
  (bind _movevalue (Timeline|Move PlayFromStart)
    (:Update
      (Utilities|AdjustPosition _movevalue))
    (:Finished
      (CallFunction|OnAttackFinished StartField TargetField))))

(event Custom|OnJumpMoveFinished
  (params (StartField :type String) (TargetField :type String) (Move :type String))
  ;[1 1 1] Attack with jump
  (bind _move (CallFunction|UpdateBoardandGetMove StartField TargetField))
  (CallFunction|InitiateNextMove _move))

(event Custom|OnAttackFinished
  (params (StartField :type String) (TargetField :type String))
  ;[1 1 1] Attack the given field (Has to be an event, because timed functions are not allowed in functions - only in  Macros)
  (bind _move (CallFunction|UpdateBoardandGetMove StartField TargetField))
  (CallFunction|InitiateNextMove _move))

(event Custom|Captured
  ;[1 1 1] On Capture, disable the collision, activate the Particle System and destroy the ChessPiece afterwards
  (Utilities|FlowControl|DoOnce false
    (:Completed
      (Collision|SetCollisionEnabled (Variables|Default|GetCollider) "NoCollision")
      (Components|Activation|SetActive (Variables|Default|GetDestroy) true false)
      (Development|SetHiddeninGame (Variables|Default|GetStaticMesh) true false)
      (Utilities|FlowControl|Delay 2.0)
      (Actor|DestroyActor))))

(event Custom|OnPawnPromotionFinished
  (params (ChessPieceToDestroy :type BP%20Self%20Playing%20Chess%20Piece%20Object%20Reference) (Move :type String))
  (Actor|DestroyActor ChessPieceToDestroy)
  (CallFunction|InitiateNextMove Move))

(event Custom|OnPawnPromotionInitiated
  (params (ChesspieceToDestroy :type BP%20Self%20Playing%20Chess%20Piece%20Object%20Reference) (FieldToSpawnOn :type BP%20Self%20Playing%20Chess%20Tile%20Object%20Reference) (Promotion :type String) (Move :type String))
  (Utilities|FlowControl|Delay 3.0)
  (bind _chesspiece (Default|SpawnChessPieceBasedonFENChar (Variables|Default|GetChess%20Board) Promotion FieldToSpawnOn))
  (bind _output_get (Variables|/Game/InteractiveMedia/SelfPlayingChess/Board/BP_SelfPlayingChessTile.BP_SelfPlayingChessTile_C|SetPresentChesspiece FieldToSpawnOn _chesspiece))
  (CallFunction|OnPawnPromotionFinished _output_get ChesspieceToDestroy Move))

(event Custom|JumpAndMove
  (params (Target :type Vector) (StartField :type String) (TargetField :type String) (Move :type String))
  ;[1 1 1] Attack with jump
  (Variables|Default|SetAttacking true)
  (bind _heighttrack (Timeline|Launch PlayFromStart)
    (:Update
      (CallFunction|AdjustHeight _heighttrack))
    (:Finished
      (CallFunction|PrepareMove Target)
      (bind _movevalue (Timeline|JumpMove PlayFromStart)
        (:Update
          (Utilities|AdjustPosition _movevalue))
        (:Finished
          (bind _heighttrack_2 (Timeline|Land PlayFromStart)
            (:Update
              (CallFunction|AdjustHeight _heighttrack_2))
            (:Finished
              (CallFunction|OnJumpMoveFinished StartField TargetField Move))))))))

(event EventBeginPlay
  (bind _returnvalue (Actor|GetActorOfClass "/Game/InteractiveMedia/SelfPlayingChess/Board/BP_SelfPlayingChessboard.BP_SelfPlayingChessboard_C"))
  (Variables|Default|SetChess%20Board _returnvalue)
  (Variables|Default|SetCollisionOffset (.z (Variables|/Script/Engine.SceneComponent|GetRelativeLocation (Variables|Default|GetCollisionRoot)))))

(event EventTick
  (params (DeltaSeconds :type Float%20%28single-precision%29))
  (Variables|Default|SetDelta%20Seconds DeltaSeconds))

(event Collision|EventActorBeginOverlap
  (params (OtherActor :type Actor%20Object%20Reference))
  ;[1 1 1] If the overlapped Actor does not have the same color and is not attacking the Chess Piece needs to be destroyed
  (bind _asbp_self_playing_chess_piece (Utilities|Casting|CastToBP_SelfPlayingChessPiece OtherActor))
  (Utilities|IsValid _asbp_self_playing_chess_piece
    (:Is%20Valid
      (if (and (!= (Variables|BP_SelfPlayingChessPiece_C|GetColor _asbp_self_playing_chess_piece) (Rendering|Material|GetMaterial (Variables|Default|GetStaticMesh) 0)) (not (Variables|Default|GetAttacking)))
        (CallFunction|Captured)))))

(fn ConstructionScript
  (Rendering|Material|SetMaterial (Variables|Default|GetStaticMesh) 0 (Variables|Default|GetColor)))

(fn InitiateNextMove
  (params (Move :type String))
  (Variables|Default|SetAttacking false)
  (Default|StartNextMove (Variables|Default|GetChess%20Board) Move))

(fn UpdateBoardandGetMove
  (params (StartField :type String) (TargetField :type String))
  (Utilities|FlowControl|Sequence
    (:then_0
      ;[1 1 1] First we need to save the ChessPiece Reference of the starting position and then set the field to empty
      (bind _field (Utilities|GetFieldbyName StartField)
        (:Is%20Valid
          (LocalVariables|SetChessPieceToMove (Variables|/Game/InteractiveMedia/SelfPlayingChess/Board/BP_SelfPlayingChessTile.BP_SelfPlayingChessTile_C|GetPresentChesspiece _field))
          (Variables|/Game/InteractiveMedia/SelfPlayingChess/Board/BP_SelfPlayingChessTile.BP_SelfPlayingChessTile_C|SetPresentChesspiece _field 0))))
    (:then_1
      ;[1 1 1] Then we need to set the ChessPiece at the target field to the one from the starting position
      (bind _field_2 (Utilities|GetFieldbyName TargetField)
        (:Is%20Valid
          (Variables|/Game/InteractiveMedia/SelfPlayingChess/Board/BP_SelfPlayingChessTile.BP_SelfPlayingChessTile_C|SetPresentChesspiece _field_2 (LocalVariables|GetChessPieceToMove)))))
    (:then_2
      (return (Utilities|String|Append " moves " StartField TargetField)))))

(fn AdjustHeight
  (params (Height :type Float%20%28double-precision%29))
  (bind _collisionroot (Variables|Default|GetCollisionRoot))
  (bind _relativelocation (Variables|/Script/Engine.SceneComponent|GetRelativeLocation _collisionroot))
  (Transformation|SetRelativeLocation (Variables|Default|GetCollisionRoot) (Math|Vector|MakeVector (.x _relativelocation) (.y _relativelocation) (+ (Variables|Default|GetCollisionOffset) Height)) false false))

(fn UpdateFieldsonCastling
  (params (StartField :type String) (TargetField :type String))
  (bind _field (Utilities|GetFieldbyName StartField)
    (:Is%20Valid
      (bind _field_2 (Utilities|GetFieldbyName TargetField)
        (:Is%20Valid
          (Variables|/Game/InteractiveMedia/SelfPlayingChess/Board/BP_SelfPlayingChessTile.BP_SelfPlayingChessTile_C|SetPresentChesspiece _field_2 (Variables|/Game/InteractiveMedia/SelfPlayingChess/Board/BP_SelfPlayingChessTile.BP_SelfPlayingChessTile_C|GetPresentChesspiece _field))
          (Variables|/Game/InteractiveMedia/SelfPlayingChess/Board/BP_SelfPlayingChessTile.BP_SelfPlayingChessTile_C|SetPresentChesspiece _field (Variables|/Game/InteractiveMedia/SelfPlayingChess/Board/BP_SelfPlayingChessTile.BP_SelfPlayingChessTile_C|GetPresentChesspiece _field_2))
          (return (Utilities|String|Append " moves " StartField TargetField)))))))

(fn PrepareMove
  (params (Target :type Vector))
  (bind _returnvalue (Transformation|GetActorLocation))
  (bind _returnvalue_2 (Transformation|GetActorRotation))
  (Variables|Default|SetStart _returnvalue)
  (Variables|Default|SetDistance (- Target _returnvalue))
  (Transformation|SetActorRotation (Math|Rotator|MakeRotator (.roll _returnvalue_2) (.pitch _returnvalue_2) (.yaw (Math|Rotator|FindLookatRotation (Variables|Default|GetStart) Target)))))