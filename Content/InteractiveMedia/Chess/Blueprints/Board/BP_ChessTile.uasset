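; BP_ChessTile is a clickable chessboard square that highlights legal moves and handles move selection.
; Cursor and click events step a shared state in the chess GameState through hover, start selection, target selection and attack initiation, while other mouse buttons back out.
; Move strings resolve to target tiles through the board's field map, and each state's material comes from a lookup map.
; The construction script labels the tile with its field name.
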(event OnEndCursorOver(Tile)
  (params (TouchedComponent :type Primitive%20Component%20Object%20Reference))
  (Utilities|CheckforCorrectState "NewEnumerator0"
    (:True
      (CallFunction|SetMarked "NewEnumerator3")
      (CallFunction|SetAllLegalMovesMarked "NewEnumerator3"))))

(event OnBeginCursorOver(Tile)
  (params (TouchedComponent :type Primitive%20Component%20Object%20Reference))
  (Utilities|CheckforCorrectState "NewEnumerator3"
    (:True
      (CallFunction|SetMarked "NewEnumerator0")
      (CallFunction|SetAllLegalMovesMarked "NewEnumerator0"))))

(event OnClicked(Tile)
  (params (TouchedComponent :type Primitive%20Component%20Object%20Reference) (ButtonPressed :type Key%20Structure :default "None"))
  (bind _gamestatechess (Variables|Default|GetGameStateChess))
  (if (== ButtonPressed "LeftMouseButton")
    ;[1 1 1] If we hover over the Tile we want to select it by clicking. If we click onto it when we are already in selection mode, we want to deselect it by clicking
    (Utilities|CheckforCorrectState "NewEnumerator0"
      (:True
        (CallFunction|SetAllLegalMovesMarked "NewEnumerator1")
        (Variables|/Game/InteractiveMedia/Chess/Blueprints/BP_GameStateChess.BP_GameStateChess_C|SetCurrentStart _gamestatechess (Variables|Default|GetFieldName))
        (Variables|/Game/InteractiveMedia/Chess/Blueprints/BP_GameStateChess.BP_GameStateChess_C|SetLegalMoves _gamestatechess (Variables|Default|GetLegalMoves)))
      (:false
        ;[1 1 1] If we already selected the start tile, we now want to set the target tile by clicking
        (Utilities|CheckforCorrectState "NewEnumerator1"
          (:True
            (bind _found (CallFunction|CheckifMoveinLegalMoves))
            (if _found
              (Variables|/Game/InteractiveMedia/Chess/Blueprints/BP_GameStateChess.BP_GameStateChess_C|SetCurrentTarget (Variables|Default|GetGameStateChess) (Variables|Default|GetFieldName))
              (CallFunction|SetMarked "NewEnumerator2")))
          (:false
            (Utilities|CheckforCorrectState "NewEnumerator2"
              (:True
                (CallFunction|ResetAllTiles)
                (Default|InitiateAttack (Variables|Default|GetGameStateChess))))))))
    (else
      ;[1 1 1] If we already highlighted a field, but we want to change to a different one, we need to reset all tiles
      (Utilities|CheckforCorrectState "NewEnumerator1"
        (:True
          (CallFunction|ResetAllTiles))
        (:false
          ;[1 1 1] If we already selected a target, we want to deselect it
          (Utilities|CheckforCorrectState "NewEnumerator2"
            (:True
              (Default|SetAllLegalMoves (Variables|Default|GetGameStateChess) "NewEnumerator1"))))))))

(event EventBeginPlay
  (bind _asbp_game_mode_chess (Utilities|Casting|CastToBP_GameModeChess (Game|GetGameMode)))
  (Variables|Default|SetChess%20Board (Variables|/Game/InteractiveMedia/Chess/Blueprints/BP_GameModeChess.BP_GameModeChess_C|GetChessBoard _asbp_game_mode_chess))
  (bind _asbp_game_state_chess (Utilities|Casting|CastToBP_GameStateChess (Game|GetGameState)))
  (Variables|Default|SetGameStateChess _asbp_game_state_chess))

(fn ConstructionScript
  (Rendering|Components|TextRender|SetText (Variables|Default|GetDebugText) (Utilities|Text|ToText(String) (Class|KismetStringLibrary|ToUpper (Variables|Default|GetFieldName)))))

(fn SetMarked
  (params (NewState :type SelectStates%20Enum :default "NewEnumerator0"))
  (Rendering|Material|SetMaterial (Variables|Default|GetTile) 0 (.Value (Utilities|Map|Find (LocalVariables|GetTileStates) NewState)))
  (Variables|/Game/InteractiveMedia/Chess/Blueprints/BP_GameStateChess.BP_GameStateChess_C|SetCurrentState (Variables|Default|GetGameStateChess) NewState))

(fn SetAllLegalMovesMarked
  (params (NewState :type SelectStates%20Enum :default "NewEnumerator0"))
  (for _array_element (Variables|Default|GetLegalMoves)
    (bind _targetfield (Utilities|GetTargetField _array_element)
      (:Is%20Valid
        (CallFunction|SetMarked _targetfield NewState)
        (Variables|/Game/InteractiveMedia/Chess/Blueprints/BP_GameStateChess.BP_GameStateChess_C|SetCurrentState (Variables|Default|GetGameStateChess) NewState)))))

(fn ResetAllTiles
  (bind _values (Utilities|Map|Values (Variables|/Game/InteractiveMedia/Chess/Blueprints/Board/BP_ChessBoard.BP_ChessBoard_C|GetFields (Variables|Default|GetChess%20Board))))
  (for _array_element _values
    (bind _asbp_chess_tile (Utilities|Casting|CastToBP_ChessTile _array_element))
    (CallFunction|SetMarked _asbp_chess_tile "NewEnumerator3")))

(fn CheckifMoveinLegalMoves
  (for _array_element (Variables|/Game/InteractiveMedia/Chess/Blueprints/BP_GameStateChess.BP_GameStateChess_C|GetLegalMoves (Variables|Default|GetGameStateChess))
    (if (Utilities|String|Contains _array_element (Variables|Default|GetFieldName))
      (return true)))
  (return false))