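; BP_PickBoard is a chess board actor that displays the six piece types: bishop, knight, pawn, king, queen and rook.
; The construction script applies one shared Material to slot 0 of every piece mesh.
; GetBoundaries returns the min and max of the Frame mesh asset's bounding box, without applying the component transform.
; It has no active event logic.
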(event EventBeginPlay)

(event Collision|EventActorBeginOverlap
  (params (OtherActor :type Actor%20Object%20Reference)))

(event EventTick
  (params (DeltaSeconds :type Float%20%28single-precision%29)))

(fn ConstructionScript
  (Rendering|Material|SetMaterial (Variables|Default|GetBishop) 0 (Variables|Default|GetMaterial)))

(fn GetBoundaries
  (bind _frame (Variables|Default|GetFrame))
  (bind _staticmesh (Variables|/Script/Engine.StaticMeshComponent|GetStaticMesh _frame))
  (bind _returnvalue (StaticMesh|GetBoundingBox _staticmesh))
  (return (.min _returnvalue) (.max _returnvalue)))