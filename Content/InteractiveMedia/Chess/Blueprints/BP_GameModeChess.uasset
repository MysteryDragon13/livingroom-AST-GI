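; Chess game mode that runs the turn loop and initializes the level's chessboard from a FEN string.
; Each move is appended to the FEN and sent to Stockfish at the set skill level, returning a corrected FEN, legal moves, best move and end flags.
; AI players play the best move through the GameState, while humans get legal moves on the board.
; Checkmate or an offerable draw prints a message and reloads the map.
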(event Custom|OnInitialize
  (params (FEN :type String) (SkillLevel :type Integer) (PlayerDetails :type Map%20of%20Integers%20to%20Structs))
  ;[1 1 1] This will be set via UI and will then be used to initialize the ChessBoard. The Playerdetails contain the name, the color and whether the player is an AI
  (Variables|Chess|SetFEN FEN)
  (Variables|Chess|SetSkillLevel SkillLevel)
  (Variables|Chess|SetPlayerDetails PlayerDetails)
  (Default|OnInitialize (Variables|Chess|GetChessBoard) (Variables|Chess|GetFEN)))

(event Custom|StartNextMove
  (params (Move :type String))
  ;[1 1 1] Method to handle the next move. We first set the move ("moves Move") to lowercase, then append it onto the current FEN. Afterwards we toggle the WhitesTurn, so basically the other color is now currently playing. We then send the new FEN to Stockfish and extract whether the game is over or can be finished. If not we check if the player is an AI we use the best move else we spread the possible moves onto the tiles.
  (bind _output_get (Variables|Chess|SetFEN (Utilities|String|Append (Variables|Chess|GetFEN) (Utilities|String|ToLower Move))))
  (Variables|Chess|SetWhite´s%20Turn (not (Variables|Chess|GetWhite´s%20Turn)))
  (Development|PrintString (Utilities|String|Append "FEN: " _output_get) true true "(R=0.000000,G=0.660000,B=1.000000,A=1.000000)" 5.0)
  (bind (_correctedfen _bestmove _legalmoves _ischeckmate _isdrawofferable) (Class|ChessAI|GetAIFeedback (Variables|Chess|GetSkillLevel) (Variables|Chess|GetFEN)))
  (Variables|Chess|SetFEN _correctedfen)
  (if _ischeckmate
    (bind _winnerstring (CallFunction|ConstructGameOverString))
    (Development|PrintString _winnerstring true true "(R=0.000000,G=1.000000,B=0.078088,A=1.000000)" 2e+02)
    (Utilities|FlowControl|Delay 5.0 :!label _label)
    (Game|OpenLevel(byObjectReference) "/Game/Maps/ChessMap.ChessMap")
    (elif _isdrawofferable
      (Development|PrintString (Variables|UIStrings|GetDrawOffer) true true "(R=1.000000,G=0.952188,B=0.000000,A=1.000000)" 2e+02)
      (goto _label)
      (else
        (bind _value (CallFunction|GetCurrentPlayer))
        (if (.isai? _value)
          (Utilities|FlowControl|Delay 0.2)
          (CallFunction|AdjustBestMovetoLegalMove _legalmoves _bestmove)
          (else
            (Default|ExtractLegalMoves (Variables|Chess|GetChessBoard) _legalmoves)))))))

(event EventBeginPlay
  ;[1 1 1] On Event BeginPlay, we save the Gamestate reference since we need to use it often and then initialize the Chessboard with the standard FEN - until we built the UI
  (bind _asbp_game_state_chess (Utilities|Casting|CastToBP_GameStateChess (Game|GetGameState)))
  (Variables|Chess|SetGameStateChess _asbp_game_state_chess)
  (Default|OnInitialize (Variables|Chess|GetChessBoard) (Variables|Chess|GetFEN)))

(event EventTick
  (params (DeltaSeconds :type Float%20%28single-precision%29)))

(fn ConstructionScript
  (bind _returnvalue (Actor|GetActorOfClass "/Game/InteractiveMedia/Chess/Blueprints/Board/BP_ChessBoard.BP_ChessBoard_C"))
  (Variables|Chess|SetChessBoard _returnvalue))

(fn ConstructGameOverString
  (bind _playerdetails (Variables|Chess|GetPlayerDetails))
  (bind _white_s_turn (Variables|Chess|GetWhite´s%20Turn))
  (bind _returnvalue (not _white_s_turn))
  (bind _returnvalue_2 (Math|Conversions|ToInteger(Boolean) _returnvalue))
  (bind _value (Utilities|Map|Find _playerdetails _returnvalue_2))
  (if (.isai? _value)
    (return (Variables|UIStrings|GetAIWon))
    (else
      (return (Utilities|String|Append "Congratulations " (.name _value) "! You won this amazing match!")))))

(fn AdjustBestMovetoLegalMove
  (params (LegalMoves :type Array%20of%20Strings) (BestMove :type String))
  (bind (_startfield _endfield) (Utilities|ExtractFields BestMove 0 2))
  (bind _gamestatechess (Variables|Chess|GetGameStateChess))
  (Variables|/Game/InteractiveMedia/Chess/Blueprints/BP_GameStateChess.BP_GameStateChess_C|SetLegalMoves _gamestatechess LegalMoves)
  (Variables|/Game/InteractiveMedia/Chess/Blueprints/BP_GameStateChess.BP_GameStateChess_C|SetCurrentStart _gamestatechess _startfield)
  (Variables|/Game/InteractiveMedia/Chess/Blueprints/BP_GameStateChess.BP_GameStateChess_C|SetCurrentTarget _gamestatechess _endfield)
  (Default|InitiateAttack _gamestatechess))

(fn GetCurrentPlayer
  (bind _playerdetails (Variables|Chess|GetPlayerDetails))
  (bind _white_s_turn (Variables|Chess|GetWhite´s%20Turn))
  (bind _returnvalue (Math|Conversions|ToInteger(Boolean) _white_s_turn))
  (bind (_value _returnvalue_2) (Utilities|Map|Find _playerdetails _returnvalue))
  (if _returnvalue_2
    (return _value)))