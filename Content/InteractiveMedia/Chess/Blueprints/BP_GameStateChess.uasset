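; Chess game state that tracks the selected start and target squares, the legal moves and the current phase.
; On BeginPlay it caches the board from the chess game mode and the first player controller.
; InitiateAttack disables mouse-over events, changes state and passes the board the legal move string matched by substring search on start and target.
; SetAllLegalMoves toggles legal-move marking through the start square's tile.
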(event Custom|InitiateAttack
  (Variables|/Script/Engine.PlayerController|SetbEnableMouseOverEvents (Variables|Default|GetPlayerController) false)
  (Variables|Default|SetCurrentState "NewEnumerator4")
  (bind _legalmove (CallFunction|GetActualMovefromLegalMoves))
  (Default|InitiateAttack (Variables|Default|GetChess%20Board) _legalmove))

(event EventBeginPlay
  (bind _asbp_game_mode_chess (Utilities|Casting|CastToBP_GameModeChess (Game|GetGameMode)))
  (Variables|Default|SetChess%20Board (Variables|/Game/InteractiveMedia/Chess/Blueprints/BP_GameModeChess.BP_GameModeChess_C|GetChessBoard _asbp_game_mode_chess))
  (bind _asbp_player_controller_chess (Utilities|Casting|CastToBP_PlayerControllerChess (Game|GetPlayerController 0)))
  (Variables|Default|SetPlayerController _asbp_player_controller_chess))

(fn ConstructionScript)

(fn SetAllLegalMoves
  (params (NewState :type SelectStates%20Enum :default "NewEnumerator3"))
  (bind _asbp_chess_tile (Utilities|Casting|CastToBP_ChessTile (.Value (Utilities|Map|Find (Variables|/Game/InteractiveMedia/Chess/Blueprints/Board/BP_ChessBoard.BP_ChessBoard_C|GetFields (Variables|Default|GetChess%20Board)) (Variables|Default|GetCurrentStart)))))
  (Default|SetAllLegalMovesMarked _asbp_chess_tile NewState))

(fn GetActualMovefromLegalMoves
  (for _array_element (Variables|Default|GetLegalMoves)
    (LocalVariables|SetMove _array_element)
    (if (and (Utilities|String|Contains _array_element (Variables|Default|GetCurrentStart)) (Utilities|String|Contains _array_element (Variables|Default|GetCurrentTarget) false true))
      (return (LocalVariables|GetMove)))))