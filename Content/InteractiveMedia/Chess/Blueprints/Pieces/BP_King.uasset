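; King piece Blueprint for the chess game, extending the piece move logic with castling.
; Castle stores the rook and its move data, then sends the king to its target square through Attack.
; When that move finishes, the king updates the board and gets the move.
; If castling, it passes that move to the rook's TowerAttack to complete the castle; otherwise it initiates the next move itself.
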(event EventBeginPlay
  (|CallParentFunction) ; This node is disabled and will not be called.\nDrag off pins to build functionality.
)

(event Collision|EventActorBeginOverlap
  (params (OtherActor :type Actor%20Object%20Reference))
  (|CallParentFunction OtherActor) ; This node is disabled and will not be called.\nDrag off pins to build functionality.
)

(event EventTick
  (params (DeltaSeconds :type Float%20%28single-precision%29))
  (|CallParentFunction DeltaSeconds) ; This node is disabled and will not be called.\nDrag off pins to build functionality.
)

(event EventCastle
  (params (Rook :type BP%20Chess%20Piece%20Object%20Reference) (TargetLocationRook :type Vector :default "0, 0, 0") (StartSquareRook :type String) (TargetSquareRook :type String) (TargetLocationKing :type Vector :default "0, 0, 0") (StartSquareKing :type String) (TargetSquareKing :type String) (Move :type String))
  (Utilities|FlowControl|Sequence
    (:then_0
      (Variables|Default|SetCastling? true)
      (Variables|Default|SetRook Rook)
      (Variables|Default|SetTarget%20Location%20Rook TargetLocationRook)
      (Variables|Default|SetStart%20Square%20Rook StartSquareRook)
      (Variables|Default|SetTarget%20Square%20Rook TargetSquareRook))
    (:then_1
      (CallFunction|Attack TargetLocationKing StartSquareKing TargetSquareKing))))

(event EventOnAttackFinished
  (params (StartField :type String) (TargetField :type String))
  (if (Variables|Default|GetCastling?)
    (Variables|Default|SetCastling? false)
    (bind _move (CallFunction|UpdateBoardandGetMove StartField TargetField))
    (bind _asbp_rook (Utilities|Casting|CastToBP_Rook (Variables|Default|GetRook)))
    (Default|TowerAttack _asbp_rook (Variables|Default|GetTarget%20Location%20Rook) (Variables|Default|GetStart%20Square%20Rook) (Variables|Default|GetTarget%20Square%20Rook) _move)
    (else
      (bind _move_2 (CallFunction|UpdateBoardandGetMove StartField TargetField))
      (CallFunction|InitiateNextMove _move_2))))

(fn ConstructionScript
  (|CallParentFunction))