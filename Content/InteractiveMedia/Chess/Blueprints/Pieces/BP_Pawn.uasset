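; Pawn piece for the chess game, adding en passant and promotion to the move and attack flow.
; EnPassant and PawnPromotion store their state ("x" means none) and start an attack; OnAttackFinished then selects the matching board update.
; En passant captures the bypassed piece, with eligibility checked against the game mode's FEN.
; Promotion shows a selection widget to humans, skips it for AI, then despawns the pawn and signals the replacement spawn.
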(event Custom|PawnPromotion
  (params (Destination :type Vector) (StartSquare :type String) (TargetSquare :type String) (Promotion :type String))
  (Variables|Default|SetPromotion Promotion)
  (CallFunction|Attack Destination StartSquare TargetSquare))

(event Custom|EnPassant
  (params (Destination :type Vector) (StartSquare :type String) (TargetSquare :type String) (EnPassantSquare :type String))
  (Variables|Default|SetEnPassantSquare EnPassantSquare)
  (CallFunction|Attack Destination StartSquare TargetSquare))

(event Custom|PromotionChosen
  (params (Promotion :type String) (StartField :type String) (TargetField :type String) (Widget :type BP%20Promotion%20Selection%20Widget%20Object%20Reference))
  (Utilities|FlowControl|Delay 1.0)
  (Widget|RemovefromParent Widget)
  (Variables|Default|SetPromotion Promotion)
  (CallFunction|UpdateBoardonPawnPromotion StartField TargetField))

(event EventBeginPlay
  (|CallParentFunction) ; This node is disabled and will not be called.\nDrag off pins to build functionality.
)

(event Collision|EventActorBeginOverlap
  (params (OtherActor :type Actor%20Object%20Reference))
  (|CallParentFunction OtherActor) ; This node is disabled and will not be called.\nDrag off pins to build functionality.
)

(event EventTick
  (params (DeltaSeconds :type Float%20%28single-precision%29))
  (|CallParentFunction DeltaSeconds) ; This node is disabled and will not be called.\nDrag off pins to build functionality.
)

(event EventOnAttackFinished
  (params (StartField :type String) (TargetField :type String))
  (if (Utilities|Enum|NotEqual(Enum) (Variables|Default|GetEnPassantSquare) "x")
    (bind _move (CallFunction|UpdateBoardonEnPassant StartField TargetField))
    (Variables|Default|SetEnPassantSquare "x")
    (CallFunction|InitiateNextMove _move)
    (elif (Utilities|Enum|NotEqual(Enum) (Variables|Default|GetPromotion) "x")
      (CallFunction|ShowPromotionifPlayer StartField TargetField)
      (else
        (bind _move_2 (CallFunction|UpdateBoardandGetMove StartField TargetField))
        (CallFunction|InitiateNextMove _move_2)))))

(fn ConstructionScript
  (|CallParentFunction))

(fn CheckforEnPassant
  (params (TargetField :type String))
  (bind _chess_board (Variables|Default|GetChess%20Board))
  (bind _asbp_game_mode_chess (Utilities|Casting|CastToBP_GameModeChess (Game|GetGameMode)))
  (bind _enpassanttarget (Class|ChessAI|ParseFEN (Variables|/Game/InteractiveMedia/Chess/Blueprints/BP_GameModeChess.BP_GameModeChess_C|GetFEN _asbp_game_mode_chess)))
  (bind (_letterindex _numberindex) (Default|ConvertFieldtoIndex _chess_board (Class|KismetStringLibrary|ToUpper _enpassanttarget)))
  (bind (_letterindex_2 _numberindex_2) (Default|ConvertFieldtoIndex _chess_board TargetField))
  (if (Variables|/Game/InteractiveMedia/Chess/Blueprints/BP_GameModeChess.BP_GameModeChess_C|GetWhite´s%20Turn _asbp_game_mode_chess)
    (return (and (== _letterindex_2 _letterindex) (== (+ _numberindex 1) _numberindex_2)) (Class|KismetStringLibrary|ToUpper _enpassanttarget))
    (else
      (return (and (== _letterindex_2 _letterindex) (== (- _numberindex 1) _numberindex_2)) (Class|KismetStringLibrary|ToUpper _enpassanttarget)))))

(fn UpdateBoardonEnPassant
  (params (StartField :type String) (TargetField :type String))
  (Utilities|FlowControl|Sequence
    (:then_0
      ;[1 1 1] First we need to save the ChessPiece Reference of the starting position and then set the field to empty
      (bind _field (Utilities|GetSquarebyName StartField)
        (:Is%20Valid
          (bind _asbp_chess_piece (Utilities|Casting|CastToBP_ChessPiece (Variables|/Game/InteractiveMedia/Chess/Blueprints/Board/BP_ChessTile.BP_ChessTile_C|GetPresentChesspiece _field)))
          (LocalVariables|SetChessPieceToMove _asbp_chess_piece)
          (Variables|/Game/InteractiveMedia/Chess/Blueprints/Board/BP_ChessTile.BP_ChessTile_C|SetPresentChesspiece _field 0))))
    (:then_1
      ;[1 1 1] Then we need to set the ChessPiece at the target field to the one from the starting position
      (bind _field_2 (Utilities|GetSquarebyName TargetField)
        (:Is%20Valid
          (Variables|/Game/InteractiveMedia/Chess/Blueprints/Board/BP_ChessTile.BP_ChessTile_C|SetPresentChesspiece _field_2 (LocalVariables|GetChessPieceToMove)))))
    (:then_2
      ;[1 1 1] Together with the move we need to trigger the captured event for the EnPassant field
      (bind _field_3 (Utilities|GetSquarebyName (Variables|Default|GetEnPassantSquare))
        (:Is%20Valid
          (bind _asbp_chess_piece_2 (Utilities|Casting|CastToBP_ChessPiece (Variables|/Game/InteractiveMedia/Chess/Blueprints/Board/BP_ChessTile.BP_ChessTile_C|GetPresentChesspiece _field_3)))
          (Default|Captured _asbp_chess_piece_2)
          (Variables|/Game/InteractiveMedia/Chess/Blueprints/Board/BP_ChessTile.BP_ChessTile_C|SetPresentChesspiece _field_3 0))))
    (:then_3
      (return (Utilities|String|Append " moves " StartField TargetField)))))

(fn UpdateBoardonPawnPromotion
  (params (StartField :type String) (TargetField :type String%20%28by%20ref%29))
  ;[1 1 1] We just need to set the ChessPiece on the starting field to empty, the rest will be handled by the event
  (bind _field (Utilities|GetSquarebyName StartField)
    (:Is%20Valid
      (Variables|/Game/InteractiveMedia/Chess/Blueprints/Board/BP_ChessTile.BP_ChessTile_C|SetPresentChesspiece _field 0)
      (Components|Activation|SetActive (Variables|Default|GetDespawn) true false)
      (bind _field_2 (Utilities|GetSquarebyName TargetField)
        (:Is%20Valid
          (CallFunction|OnPawnPromotionInitiated self _field_2 (Variables|Default|GetPromotion) (Utilities|String|Append " moves " StartField TargetField (Variables|Default|GetPromotion))))))))

(fn ShowPromotionifPlayer
  (params (StartField :type String) (TargetField :type String))
  (bind _asbp_game_mode_chess (Utilities|Casting|CastToBP_GameModeChess (Game|GetGameMode)))
  (bind _value (Default|GetCurrentPlayer _asbp_game_mode_chess))
  (if (.isai? _value)
    (CallFunction|UpdateBoardonPawnPromotion StartField TargetField)
    (else
      (bind _returnvalue (Game|ConstructObjectfromClass "/Game/InteractiveMedia/Chess/Blueprints/BP_PromotionSelectionWidget.BP_PromotionSelectionWidget_C"))
      (Default|SetImages _returnvalue self (.white? _value) StartField TargetField)
      (UserInterface|Viewport|AddtoViewport _returnvalue 0))))