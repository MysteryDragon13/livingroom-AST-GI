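; Base chess piece that moves across the board by AI movement, with empty events for en passant, promotion and castling.
; Attacks and timeline-driven jumps retry failed moves, then update tile occupancy and pass a move string to the game mode.
; Overlapping a differently colored piece while not attacking triggers capture: particles, hidden mesh, delayed destruction.
; A promotion handler replaces the piece with one spawned from a FEN character.
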(event Custom|Castle
  (params (Rook :type BP%20Chess%20Piece%20Object%20Reference) (TargetLocationRook :type Vector) (StartSquareRook :type String) (TargetSquareRook :type String) (TargetLocationKing :type Vector) (StartSquareKing :type String) (TargetSquareKing :type String) (Move :type String))
  ;[1 1 1] Events for Special Cases
)

(event Custom|EnPassant
  (params (Destination :type Vector) (StartSquare :type String) (TargetSquare :type String) (EnPassantSquare :type String))
  ;[1 1 1] Events for Special Cases
)

(event Custom|PawnPromotion
  (params (Destination :type Vector) (StartSquare :type String) (TargetSquare :type String) (Promotion :type String))
  ;[1 1 1] Events for Special Cases
)

(event Custom|Attack
  (params (Target :type Vector) (StartField :type String) (TargetField :type String))
  ;[1 1 1] Attack the given field (Has to be an event, because timed functions are not allowed in functions - only in  Macros)
  (Variables|Default|SetAttacking true)
  (AI|AIMoveTo self Target 0 5.0 false :!label _label
    (:OnSuccess
      (CallFunction|OnAttackFinished StartField TargetField))
    (:OnFail
      (Utilities|FlowControl|RetriggerableDelay 0.2)
      (goto _label))))

(event Custom|OnJumpMoveFinished
  (params (StartField :type String) (TargetField :type String) (Move :type String))
  ;[1 1 1] Attack with jump
  (bind _move (Lesson7:MoveSelection|UpdateBoardandGetMove StartField TargetField))
  (Lesson7:MoveSelection|InitiateNextMove _move))

(event Custom|OnAttackFinished
  (params (StartField :type String) (TargetField :type String))
  ;[1 1 1] Attack the given field (Has to be an event, because timed functions are not allowed in functions - only in  Macros)
  (bind _move (Lesson7:MoveSelection|UpdateBoardandGetMove StartField TargetField))
  (Lesson7:MoveSelection|InitiateNextMove _move))

(event Custom|Captured
  ;[1 1 1] On Capture, disable the collision, activate the Particle System and destroy the ChessPiece afterwards
  (Utilities|FlowControl|DoOnce false
    (:Completed
      (Collision|SetCollisionEnabled (Variables|Default|GetCollider) "NoCollision")
      (Components|Activation|SetActive (Variables|Default|GetDestroy) true false)
      (Development|SetHiddeninGame (Variables|Default|GetStaticMesh) true false)
      (Utilities|FlowControl|Delay 2.0)
      (Actor|DestroyActor))))

(event Custom|OnPawnPromotionInitiated
  (params (ChesspieceToDestroy :type BP%20Chess%20Piece%20Object%20Reference) (FieldToSpawnOn :type BP%20Chess%20Tile%20Object%20Reference) (Promotion :type String) (Move :type String))
  (Utilities|FlowControl|Delay 3.0)
  (Actor|DestroyActor ChesspieceToDestroy)
  (bind _returnvalue (Default|SpawnChessPieceBasedonFENChar (Variables|Default|GetChess%20Board) Promotion (Transformation|GetActorLocation FieldToSpawnOn)))
  (bind _asbp_chess_piece (Utilities|Casting|CastToBP_ChessPiece _returnvalue))
  (Variables|/Game/InteractiveMedia/Chess/Blueprints/Board/BP_ChessTile.BP_ChessTile_C|SetPresentChesspiece FieldToSpawnOn _asbp_chess_piece)
  (Lesson7:MoveSelection|InitiateNextMove Move))

(event Custom|JumpAndMove
  (params (Target :type Vector) (StartField :type String) (TargetField :type String) (Move :type String))
  ;[1 1 1] Attack with jump
  (Variables|Default|SetAttacking true)
  (bind _heighttrack (Timeline|Timeline PlayFromStart)
    (:Update
      (Lesson8:AIMovement|AdjustHeight _heighttrack))
    (:Finished
      (AI|AIMoveTo self Target 0 5.0 false :!label _label
        (:OnSuccess
          (bind _heighttrack_2 (Timeline|Timeline_0 PlayFromStart)
            (:Update
              (Lesson8:AIMovement|AdjustHeight _heighttrack_2))
            (:Finished
              (CallFunction|OnJumpMoveFinished StartField TargetField Move))))
        (:OnFail
          (Utilities|FlowControl|RetriggerableDelay 0.2)
          (goto _label))))))

(event EventBeginPlay
  (bind _asbp_game_mode_chess (Utilities|Casting|CastToBP_GameModeChess (Game|GetGameMode)))
  (Variables|Default|SetChess%20Board (Variables|/Game/InteractiveMedia/Chess/Blueprints/BP_GameModeChess.BP_GameModeChess_C|GetChessBoard _asbp_game_mode_chess))
  (Variables|Default|SetCollisionOffset (.z (Variables|/Script/Engine.SceneComponent|GetRelativeLocation (Variables|Default|GetCollisionRoot)))))

(event EventTick
  (params (DeltaSeconds :type Float%20%28single-precision%29)))

(event Collision|EventActorBeginOverlap
  (params (OtherActor :type Actor%20Object%20Reference))
  ;[1 1 1] If the overlapped Actor does not have the same color and is not attacking the Chess Piece needs to be destroyed
  (bind _asbp_chess_piece (Utilities|Casting|CastToBP_ChessPiece OtherActor))
  (Utilities|IsValid _asbp_chess_piece
    (:Is%20Valid
      (if (and (!= (Rendering|Material|GetMaterial (Variables|BP_ChessPiece_C|GetStaticMesh _asbp_chess_piece) 0) (Rendering|Material|GetMaterial (Variables|Default|GetStaticMesh) 0)) (not (Variables|Default|GetAttacking)))
        (CallFunction|Captured)))))

(fn ConstructionScript)

(fn InitiateNextMove
  (params (Move :type String))
  (Variables|Default|SetAttacking false)
  (bind _asbp_game_mode_chess (Utilities|Casting|CastToBP_GameModeChess (Game|GetGameMode)))
  (bind _asbp_game_state_chess (Utilities|Casting|CastToBP_GameStateChess (Game|GetGameState)))
  (Variables|/Game/InteractiveMedia/Chess/Blueprints/BP_GameStateChess.BP_GameStateChess_C|SetCurrentState _asbp_game_state_chess "NewEnumerator3")
  (Default|StartNextMove _asbp_game_mode_chess Move))

(fn UpdateBoardandGetMove
  (params (StartField :type String) (TargetField :type String))
  (Utilities|FlowControl|Sequence
    (:then_0
      ;[1 1 1] First we need to save the ChessPiece Reference of the starting position and then set the field to empty
      (bind _field (Utilities|GetFieldbyName StartField)
        (:Is%20Valid
          (bind _asbp_chess_piece (Utilities|Casting|CastToBP_ChessPiece (Variables|/Game/InteractiveMedia/Chess/Blueprints/Board/BP_ChessTile.BP_ChessTile_C|GetPresentChesspiece _field)))
          (LocalVariables|SetChessPieceToMove _asbp_chess_piece)
          (Variables|/Game/InteractiveMedia/Chess/Blueprints/Board/BP_ChessTile.BP_ChessTile_C|SetPresentChesspiece _field 0))))
    (:then_1
      ;[1 1 1] Then we need to set the ChessPiece at the target field to the one from the starting position
      (bind _field_2 (Utilities|GetFieldbyName TargetField)
        (:Is%20Valid
          (Variables|/Game/InteractiveMedia/Chess/Blueprints/Board/BP_ChessTile.BP_ChessTile_C|SetPresentChesspiece _field_2 (LocalVariables|GetChessPieceToMove)))))
    (:then_2
      (return (Utilities|String|Append " moves " StartField TargetField)))))

(fn AdjustHeight
  (params (Height :type Float%20%28double-precision%29))
  (bind _collisionroot (Variables|Default|GetCollisionRoot))
  (bind _relativelocation (Variables|/Script/Engine.SceneComponent|GetRelativeLocation _collisionroot))
  (Transformation|SetRelativeLocation (Variables|Default|GetCollisionRoot) (Math|Vector|MakeVector (.x _relativelocation) (.y _relativelocation) (+ (Variables|Default|GetCollisionOffset) Height)) false false))

(fn UpdateFieldsonCastling
  (params (StartField :type String) (TargetField :type String))
  (bind _field (Utilities|GetFieldbyName StartField)
    (:Is%20Valid
      (bind _field_2 (Utilities|GetFieldbyName TargetField)
        (:Is%20Valid
          (Variables|/Game/InteractiveMedia/Chess/Blueprints/Board/BP_ChessTile.BP_ChessTile_C|SetPresentChesspiece _field_2 (Variables|/Game/InteractiveMedia/Chess/Blueprints/Board/BP_ChessTile.BP_ChessTile_C|GetPresentChesspiece _field))
          (Variables|/Game/InteractiveMedia/Chess/Blueprints/Board/BP_ChessTile.BP_ChessTile_C|SetPresentChesspiece _field (Variables|/Game/InteractiveMedia/Chess/Blueprints/Board/BP_ChessTile.BP_ChessTile_C|GetPresentChesspiece _field_2))
          (return (Utilities|String|Append " moves " StartField TargetField)))))))